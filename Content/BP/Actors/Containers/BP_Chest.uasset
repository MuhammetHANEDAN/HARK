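; Chest container actor that shows a prompt and highlight when interaction begins.
; Interact shows the message widget component and applies an outline overlay material to the skeletal mesh.
; InteractEnd hides the widget and clears the overlay.
; Open and close animation calls exist in the graph but are unconnected, so the chest never animates from this logic.
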(event EventBeginPlay)

(event Collision|EventActorBeginOverlap
  (params (OtherActor :type Actor%20Object%20Reference)))

(event EventTick
  (params (DeltaSeconds :type Float%20%28single-precision%29)))

(event EventInteract
  (Rendering|SetVisibility (Variables|Default|GetShowMessageWidgetComponent) true false)
  (Rendering|Material|SetOverlayMaterial (Variables|Default|GetSkeletalMesh) "/Game/Assets/Materials/M_OutLine.M_OutLine" :!class /Script/Engine.MeshComponent))

(event EventInteractEnd
  (Rendering|SetVisibility (Variables|Default|GetShowMessageWidgetComponent) false false)
  (Rendering|Material|SetOverlayMaterial (Variables|Default|GetSkeletalMesh) 0 :!class /Script/Engine.MeshComponent))

(fn ConstructionScript)